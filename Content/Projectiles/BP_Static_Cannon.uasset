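; BP_Static_Cannon is a stationary cannon that periodically fires projectiles in a fixed direction.
; On BeginPlay it picks one random interval and starts a looping timer, which plays an attenuated fire sound and spawns a BP_Bullet at the InitialDirection component's transform.
; Player-tracking and aiming logic remains in the graph but is disconnected, so Tick does nothing and the cannon never turns itself.
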(event `self.ReceiveBeginPlay`
  (set `self.Random time` (`KismetMathLibrary.RandomFloatInRange` 5.0 10.0))
  (`KismetSystemLibrary.K2_SetTimerDelegate` (delegate `cannon_fire`) (`self.Random time`) true))

(event `cannon_fire`
  ;[1 0.501 0.3707] Firing canon
  (`GameplayStatics.PlaySoundAtLocation` "/Game/SoundFX/Cannon/CannonFire.CannonFire" (`SceneComponent.K2_GetComponentLocation` (`self.Cannon_Base`)) (struct) 0.15 1.0 0.0 "/Game/Projectiles/Cannon.Cannon" null null)
  (`|SpawnActorFromClass` "/Game/Projectiles/BP_Bullet.BP_Bullet_C" (`SceneComponent.K2_GetComponentToWorld` (`self.InitialDirection`)) "Undefined" "OverrideRootScale" null null))

(event `self.ReceiveTick`
  (params (DeltaSeconds :type "Float (single-precision)"))
  ;[0.1521 1 0.477] Look At PLayer
)

(event `AimAtTarget`
  (bind _returnvalue (`KismetMathLibrary.MakeRotFromX` (`KismetMathLibrary.InverseTransformDirection` (`self.GetTransform`) (- (`self.target location`) (`SceneComponent.K2_GetComponentLocation` (`self.Cannon`))))))
  ;[1 1 1] Original Code - Not in use
  (`SceneComponent.K2_SetRelativeRotation` (`self.Cannon_Base`) (`KismetMathLibrary.RInterpTo_Constant` (`SceneComponent.RelativeRotation` (`self.Cannon_Base`)) (`KismetMathLibrary.MakeRotator` 0.0 0.0 (.yaw _returnvalue)) (`GameplayStatics.GetWorldDeltaSeconds`)) false false)
  (`SceneComponent.K2_SetRelativeRotation` (`self.Cannon`) (`KismetMathLibrary.RInterpTo_Constant` (`SceneComponent.RelativeRotation` (`self.Cannon`)) (`KismetMathLibrary.MakeRotator` 0.0 (.pitch _returnvalue)) (`GameplayStatics.GetWorldDeltaSeconds`)) false false))

(event `ResetAim`
  ;[1 1 1] Original Code - Not in use
)

(event `Target_player`
  ;[1 1 1] Original Code - Not in use
)

(fn `UserConstructionScript`)