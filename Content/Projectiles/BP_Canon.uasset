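; BP_Canon is a cannon actor that aims at the first BP_Target found in the level on BeginPlay.
; Each Tick it checks the target's distance, calling AimAtTarget within range and an empty ResetAim otherwise.
; Aiming converts the target direction to actor-local space, then uses RInterpToConstant to turn CannonBase in yaw and Cannon in pitch separately.
; Firing and BP_Bullet spawning are present but unconnected, so it never shoots.
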(event `self.ReceiveTick`
  (params (DeltaSeconds :type "Float (single-precision)"))
  ;[1 1 1] Get Target Location
  (set `self.TargetLocation` (`self.K2_GetActorLocation` (`self.Target`)))
  ;[1 1 1] Check Target Distance
  (if (<= (`KismetMathLibrary.VSize` (- (`self.K2_GetActorLocation`) (`self.TargetLocation`))) 1000.0)
    (`self.AimAtTarget`)
    (else
      (`self.ResetAim`))))

(event `AimAtTarget`
  (bind _returnvalue (`KismetMathLibrary.MakeRotFromX` (`KismetMathLibrary.InverseTransformDirection` (`self.GetTransform`) (- (`self.TargetLocation`) (`SceneComponent.K2_GetComponentLocation` (`self.Cannon`))))))
  (`SceneComponent.K2_SetRelativeRotation` (`self.Cannon_Base`) (`KismetMathLibrary.RInterpTo_Constant` (`SceneComponent.RelativeRotation` (`self.Cannon_Base`)) (`KismetMathLibrary.MakeRotator` 0.0 0.0 (.yaw _returnvalue)) (`GameplayStatics.GetWorldDeltaSeconds`)) false false)
  (`SceneComponent.K2_SetRelativeRotation` (`self.Cannon`) (`KismetMathLibrary.RInterpTo_Constant` (`SceneComponent.RelativeRotation` (`self.Cannon`)) (`KismetMathLibrary.MakeRotator` 0.0 (.pitch _returnvalue)) (`GameplayStatics.GetWorldDeltaSeconds`)) false false))

(event `ResetAim`)

(event `self.ReceiveBeginPlay`
  (bind _outactors (`GameplayStatics.GetAllActorsOfClass` "/Game/Projectiles/BP_Target.BP_Target_C"))
  (set `self.Target` (`|GetArrayItem` _outactors)))

(event `Target_player`)

(fn `UserConstructionScript`)