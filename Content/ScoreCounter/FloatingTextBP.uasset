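; FloatingTextBP is a short-lived floating text actor that shows a random phrase through a FloatingScore widget component.
; On BeginPlay it picks one of ten Funnys entries for the Score text and drives the widget's opacity with a Fade timeline.
; A parallel Movement timeline lerps the actor from its spawn location toward a fixed world point near the origin, not a relative offset, then destroys it.
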(event `self.ReceiveBeginPlay`
  (`|ExecutionSequence`
    (:`then_0`
      (bind _asfloating_score (cast `/Game/ScoreCounter/FloatingScore` (`WidgetComponent.GetUserWidgetObject` (`self.Widget`))))
      (`TextBlock.SetText` (`/Game/ScoreCounter/FloatingScore.Score` _asfloating_score) (`KismetTextLibrary.Conv_StringToText` (`|GetArrayItem` (`/Game/ScoreCounter/FloatingScore.Funnys` _asfloating_score) (`KismetMathLibrary.RandomIntegerInRange` 0 9))))
      (bind (_direction _fade) (`Timeline|Fade`)
        (:`Update`
          (`Widget.SetRenderOpacity` _asfloating_score _fade))))
    (:`then_1`
      (set `self.Initial Loc` (`self.K2_GetActorLocation`))
      (bind (_direction_2 _newtrack_0) (`Timeline|Movement` :!via `PlayFromStart`)
        (:`Update`
          (`self.K2_SetActorLocation` (`KismetMathLibrary.VLerp` (`self.Initial Loc`) (25.0 25.0 25.0) _newtrack_0)))
        (:`Finished`
          (`self.K2_DestroyActor`))))))

(fn `UserConstructionScript`)